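; Lantern light Blueprint for the Singapore Canal scene, with a rope and a switchable light, built entirely in the construction script.
; The script adds a rope knot mesh and a Z-forward spline mesh component within two nested loops, then applies the light switch inside them.
; LightOn drives the light's visibility and sets the lantern material when on; when off, it zeroes intensity and radius and hides the sphere in game.
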(fn `UserConstructionScript`
  (bind _light_on (`self.Light on`))
  (bind _lightcomponent0 (`self.LightComponent0`))
  ;[1 1 1] Rope Spline
  (for _ (range 1)
    (bind _returnvalue (`AddComponent|NODE_AddStaticMeshComponent-0`))
    (`SceneComponent.K2_SetRelativeRotation` :`self` _returnvalue)
    (`StaticMeshComponent.SetStaticMesh` _returnvalue "/Game/changjing/MT_TempleKit/Artworking/Meshes/Meshes_Rope/SM_RopeKnot.SM_RopeKnot")
    (for _ (range 1)
      (bind _returnvalue_2 (`AddComponent|NODE_AddSplineMeshComponent-0`))
      (`SplineMeshComponent.SetForwardAxis` _returnvalue_2 "Z" true)
      (`SplineMeshComponent.SetStartAndEnd` _returnvalue_2 (0.0 0.0 0.0) (0.0 0.0 0.0) (0.0 0.0 0.0) (0.0 0.0 0.0) true)
      ;[1 1 1] Light Switch
      (`SceneComponent.SetVisibility` _lightcomponent0 _light_on false)
      (if _light_on
        (`PrimitiveComponent.SetMaterial` (`self.SM_Lantern_01`) 0 "/Game/changjing/Singapore_Canal/Materials/MI_Lanterns_01.MI_Lanterns_01")
        (else
          (`LightComponent.SetIntensity` _lightcomponent0 0.0)
          (`LocalLightComponent.SetAttenuationRadius` _lightcomponent0 0.0)
          (`SceneComponent.SetHiddenInGame` (`self.Sphere`) true false))))))
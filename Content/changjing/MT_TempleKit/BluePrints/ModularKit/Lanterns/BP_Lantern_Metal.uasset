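; Metal temple lantern Blueprint that hangs on a spline-built rope and has a switchable light.
; The construction script puts a knot mesh at each spline point and chains spline mesh components along the length, spaced by MeshLength scaled by actor Z scale.
; LightOn sets light visibility and swaps in the emissive material when on.
; When off, it zeroes intensity and radius and hides the fake fog meshes in game.
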(fn `UserConstructionScript`
  (bind (_returnvalue_x _returnvalue_y _returnvalue_z) (`KismetMathLibrary.BreakVector` (`self.GetActorScale3D`)))
  (bind _mesh_length (`self.Mesh Length`))
  (bind _spline1 (`self.spline1`))
  (bind _spline1_2 (`self.spline1`))
  (bind _lightcomponent0 (`self.LightComponent0`))
  (bind _light_on (`self.Light on`))
  ;[1 1 1] Rope Spline
  (for _index (range (+ (`SplineComponent.GetNumberOfSplinePoints` _spline1) 1))
    (bind _returnvalue (`AddComponent|NODE_AddStaticMeshComponent-0` :`RelativeTransform` (`KismetMathLibrary.Conv_VectorToTransform` (`SplineComponent.GetLocationAtSplinePoint` _spline1 _index "Local"))))
    (`SceneComponent.K2_SetRelativeRotation` _returnvalue (`SplineComponent.GetRotationAtSplinePoint` _spline1 _index "Local") false false)
    (`StaticMeshComponent.SetStaticMesh` _returnvalue "/Game/changjing/MT_TempleKit/Artworking/Meshes/Meshes_Rope/SM_RopeKnot.SM_RopeKnot")
    (set `self.Mesh Length` (* _returnvalue_z _mesh_length))
    (for _index_2 (range (+ (`KismetMathLibrary.FTrunc` (/ (`SplineComponent.GetSplineLength` _spline1_2) _mesh_length)) 1))
      (bind _returnvalue_2 (`AddComponent|NODE_AddSplineMeshComponent-0`))
      (`SplineMeshComponent.SetForwardAxis` _returnvalue_2 "Z" true)
      (bind _returnvalue_3 (* _index_2 _mesh_length))
      (bind _returnvalue_4 (* (+ _index_2 1) _mesh_length))
      (`SplineMeshComponent.SetStartAndEnd` _returnvalue_2 (`SplineComponent.GetLocationAtDistanceAlongSpline` _spline1_2 _returnvalue_3 "Local") (`KismetMathLibrary.ClampVectorSize` (`SplineComponent.GetTangentAtDistanceAlongSpline` _spline1_2 _returnvalue_3 "Local") 0.0 _mesh_length) (`SplineComponent.GetLocationAtDistanceAlongSpline` _spline1_2 _returnvalue_4 "Local") (`KismetMathLibrary.ClampVectorSize` (`SplineComponent.GetTangentAtDistanceAlongSpline` _spline1_2 _returnvalue_4 "Local") 0.0 _mesh_length) true)
      ;[1 1 1] Light switch
      (`SceneComponent.SetVisibility` _lightcomponent0 _light_on false)
      (if _light_on
        (`PrimitiveComponent.SetMaterial` (`self.StaticMeshComponent0`) 0 "/Game/changjing/MT_TempleKit/Artworking/Materials/ModularPieces/MI_Lanterns_MetalEmiss.MI_Lanterns_MetalEmiss")
        (else
          (`LightComponent.SetIntensity` _lightcomponent0 0.0)
          (`LocalLightComponent.SetAttenuationRadius` _lightcomponent0 0.0)
          (`SceneComponent.SetHiddenInGame` (`self.SM_FakeFog`) true false)
          (`SceneComponent.SetHiddenInGame` (`self.SM_FakeFog2`) true false)
          (`SceneComponent.SetHiddenInGame` (`self.SM_FakeFog3`) true false)
          (`SceneComponent.SetHiddenInGame` (`self.SM_FakeFog4`) true false)
          (`SceneComponent.SetHiddenInGame` (`self.SM_FakeFog5`) true false)
          (`SceneComponent.SetHiddenInGame` (`self.SM_FakeFog9`) true false)
          (`SceneComponent.SetHiddenInGame` (`self.SM_FakeFog10`) true false)
          (`SceneComponent.SetHiddenInGame` (`self.SM_FakeFog1`) true false))))))
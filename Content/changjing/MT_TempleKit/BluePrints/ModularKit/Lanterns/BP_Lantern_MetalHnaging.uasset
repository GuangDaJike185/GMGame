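; A hanging metal lantern prop from a modular temple kit, with a LightOn switch for placing it lit or unlit.
; The construction script sets the light's visibility from the switch and applies an emissive metal material to the mesh when lit.
; When unlit, it also zeroes the light's intensity and attenuation radius and hides the fake-fog meshes in game.
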(fn `UserConstructionScript`
  (bind _lightcomponent1 (`self.LightComponent1`))
  (bind _light_on (`self.Light on`))
  ;[1 1 1] Ligt Switch
  (`SceneComponent.SetVisibility` _lightcomponent1 _light_on false)
  (if _light_on
    (`PrimitiveComponent.SetMaterial` (`self.StaticMeshComponent0`) 0 "/Game/changjing/MT_TempleKit/Artworking/Materials/ModularPieces/MI_Lanterns_MetalEmiss.MI_Lanterns_MetalEmiss")
    (else
      (`LightComponent.SetIntensity` _lightcomponent1 0.0)
      (`LocalLightComponent.SetAttenuationRadius` _lightcomponent1 0.0)
      (`SceneComponent.SetHiddenInGame` (`self.SM_FakeFog2`) true false)
      (`SceneComponent.SetHiddenInGame` (`self.SM_FakeFog3`) true false)
      (`SceneComponent.SetHiddenInGame` (`self.SM_FakeFog4`) true false)
      (`SceneComponent.SetHiddenInGame` (`self.SM_FakeFog5`) true false)
      (`SceneComponent.SetHiddenInGame` (`self.SM_FakeFog9`) true false)
      (`SceneComponent.SetHiddenInGame` (`self.SM_FakeFog10`) true false)
      (`SceneComponent.SetHiddenInGame` (`self.SM_FakeFog1`) true false)
      (`SceneComponent.SetHiddenInGame` (`self.SM_FakeFog`) true false))))
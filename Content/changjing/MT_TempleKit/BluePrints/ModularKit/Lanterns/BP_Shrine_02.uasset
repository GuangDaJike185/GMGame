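; BP_Shrine_02 is a temple-kit shrine lantern prop with a switchable point light, candle flame effect and fake-fog meshes.
; The construction script sets light visibility from LightOn and calls ActivateEffect when it is on.
; When off, it zeroes the light's intensity and radius and hides the fog meshes, sphere and flame in game.
; Separate events activate and deactivate the flame particles.
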(event `Activate_Effect`
  ;[1 1 1] Particle Switch
  (`ActorComponent.Activate` (`self.CandleFlame`) false))

(event `Deactivate_Effect`
  ;[1 1 1] Particle Switch
  (`ActorComponent.Deactivate` (`self.CandleFlame`)))

(fn `UserConstructionScript`
  (bind _light_on (`self.Light on`))
  (bind _pointlight (`self.PointLight`))
  ;[1 1 1] Light Switch
  (`SceneComponent.SetVisibility` (`self.PointLight`) _light_on false)
  (if _light_on
    (`self.Activate_Effect`)
    (else
      (`LightComponent.SetIntensity` _pointlight 0.0)
      (`LocalLightComponent.SetAttenuationRadius` _pointlight 0.0)
      (`SceneComponent.SetHiddenInGame` (`self.SM_FakeFog`) true false)
      (`SceneComponent.SetHiddenInGame` (`self.SM_FakeFog1`) true false)
      (`SceneComponent.SetHiddenInGame` (`self.SM_FakeFog3`) true false)
      (`SceneComponent.SetHiddenInGame` (`self.Sphere`) true false)
      (`SceneComponent.SetHiddenInGame` (`self.SM_FakeFog2`) true false)
      (`SceneComponent.SetHiddenInGame` (`self.CandleFlame`) true false))))
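; Pedestal brazier prop from the temple kit's lantern set, with a light and flame effect switched by a LightOn flag.
; The construction script sets light visibility from LightOn and calls the matching activate or deactivate effect, also zeroing intensity and attenuation radius when off.
; Activate_Effect and Deactivate_Effect events in the event graph start and stop the Flames component.
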(event `Activate_Effect`
  (`ActorComponent.Activate` (`self.Flames`) false))

(event `Deactivate_Effect`
  (`ActorComponent.Deactivate` (`self.Flames`)))

(fn `UserConstructionScript`
  (bind _lightcomponent0 (`self.LightComponent0`))
  (bind _light_on (`self.Light on`))
  (`SceneComponent.SetVisibility` (`self.LightComponent0`) _light_on false)
  (if _light_on
    (`self.Activate_Effect`)
    (else
      (`LightComponent.SetIntensity` _lightcomponent0 0.0)
      (`LocalLightComponent.SetAttenuationRadius` _lightcomponent0 0.0)
      (`self.Deactivate_Effect`))))
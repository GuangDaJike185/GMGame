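; BP_Bunting is a construction-script spline tool that lays out a rope bunting in the temple modular kit.
; It tiles a static mesh along the spline as spline mesh segments of MeshLength each, forward axis Z, with tangents clamped to that length.
; Start and end meshes snap to the first and last spline points, oriented along the tangent, and use the SM_RopeKnot mesh.
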(fn `UserConstructionScript`
  (bind _spline (`self.Spline`))
  (bind _meshlength (`self.MeshLength`))
  (bind _spline_2 (`self.Spline`))
  (bind _startmesh (`self.Startmesh`))
  (bind _endmesh (`self.Endmesh`))
  (bind (_location _tangent) (`SplineComponent.GetLocationAndTangentAtSplinePoint` _spline 0 "World"))
  (bind (_location_2 _tangent_2) (`SplineComponent.GetLocationAndTangentAtSplinePoint` _spline (- (`SplineComponent.GetNumberOfSplinePoints` _spline) 1) "World"))
  (for _index (range (+ (`KismetMathLibrary.FTrunc` (/ (`SplineComponent.GetSplineLength` _spline_2) _meshlength)) 1))
    (bind _returnvalue (`AddComponent|NODE_AddSplineMeshComponent-2`))
    (`StaticMeshComponent.SetStaticMesh` _returnvalue (`self.Static Mesh`))
    (`SplineMeshComponent.SetForwardAxis` _returnvalue "Z" true)
    (bind _returnvalue_2 (* _index _meshlength))
    (bind _returnvalue_3 (* (+ _index 1) _meshlength))
    (`SplineMeshComponent.SetStartAndEnd` _returnvalue (`SplineComponent.GetLocationAtDistanceAlongSpline` _spline_2 _returnvalue_2 "Local") (`KismetMathLibrary.ClampVectorSize` (`SplineComponent.GetTangentAtDistanceAlongSpline` _spline_2 _returnvalue_2 "Local") 0.0 _meshlength) (`SplineComponent.GetLocationAtDistanceAlongSpline` _spline_2 _returnvalue_3 "Local") (`KismetMathLibrary.ClampVectorSize` (`SplineComponent.GetTangentAtDistanceAlongSpline` _spline_2 _returnvalue_3 "Local") 0.0 _meshlength) true)
    (`SceneComponent.K2_SetWorldLocationAndRotation` _startmesh _location (`KismetMathLibrary.Conv_VectorToRotator` _tangent) false false)
    (`SceneComponent.K2_SetWorldLocationAndRotation` _endmesh _location_2 (`KismetMathLibrary.Conv_VectorToRotator` _tangent_2) false false)
    (`StaticMeshComponent.SetStaticMesh` _startmesh "/Game/changjing/MT_TempleKit/Artworking/Meshes/Meshes_Rope/SM_RopeKnot.SM_RopeKnot")
    (`StaticMeshComponent.SetStaticMesh` _endmesh "/Game/changjing/MT_TempleKit/Artworking/Meshes/Meshes_Rope/SM_RopeKnot.SM_RopeKnot")))
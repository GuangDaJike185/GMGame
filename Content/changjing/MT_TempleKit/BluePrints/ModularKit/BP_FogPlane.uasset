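; BP_FogPlane is a placeable fog plane in the MT_TempleKit modular kit, configured through variables on the actor.
; The Construction Script scales the Plane by Size, creates a dynamic instance of Material and assigns it to the plane.
; It then copies variables for colour gradient, panning, contrast, opacity, falloff and depth fades into that instance.
; The event graph is inactive, so the Blueprint adds no runtime logic.
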(fn `UserConstructionScript`
  (bind _mid_fog (`self.MID_Fog`))
  (`SceneComponent.SetRelativeScale3D` (`self.Plane`) (`self.Size`))
  (bind _returnvalue (`KismetMaterialLibrary.CreateDynamicMaterialInstance` (`self.Material`)))
  (bind _output_get (set `self.MID_Fog` _returnvalue))
  (`PrimitiveComponent.SetMaterial` (`self.Plane`) 0 _output_get)
  (`MaterialInstanceDynamic.SetScalarParameterValue` _mid_fog "TopColourFalloff" (`self.TopColourFalloff`))
  (`MaterialInstanceDynamic.SetScalarParameterValue` _mid_fog "TopColourPosition" (`self.TopColourPosition`))
  (`MaterialInstanceDynamic.SetVectorParameterValue` _mid_fog "Colour Top" (`self.Colour Top`))
  (`MaterialInstanceDynamic.SetVectorParameterValue` _mid_fog "Colour Bottom" (`self.Colour Bottom`))
  (`MaterialInstanceDynamic.SetScalarParameterValue` _mid_fog "PanningSpeed" (`self.PanningSpeed`))
  (`MaterialInstanceDynamic.SetScalarParameterValue` _mid_fog "Contrast" (`self.Contrast`))
  (`MaterialInstanceDynamic.SetScalarParameterValue` _mid_fog "ClippingFadeDistance" (`self.ClippingFadeDistance`))
  (`MaterialInstanceDynamic.SetScalarParameterValue` _mid_fog "FalloffExponent" (`self.FalloffExponent`))
  (`MaterialInstanceDynamic.SetScalarParameterValue` _mid_fog "MaxOpacity" (`self.MaxOpacity`))
  (`MaterialInstanceDynamic.SetScalarParameterValue` _mid_fog "CameraDepthDistance" (`self.CameraDepthDistance`))
  (`MaterialInstanceDynamic.SetScalarParameterValue` _mid_fog "CameraDepthFade" (`self.CameraDepthFade`)))
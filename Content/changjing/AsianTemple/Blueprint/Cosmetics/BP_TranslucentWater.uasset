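; BP_TranslucentWater is a configurable translucent water surface actor for the AsianTemple environment.
; On construction, it creates a dynamic instance of the ocean material on a static mesh and scales that mesh in X and Y.
; It then pushes the exposed color, depth, wave, opacity and scale variables into the material, along with the mesh's world Z as water height.
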(fn `UserConstructionScript`
  (bind _sm_watersurface (`self.SM_WaterSurface`))
  (bind _water_material (`self.Water Material`))
  (bind _water_material_2 (`self.Water Material`))
  (bind _returnvalue (`PrimitiveComponent.CreateDynamicMaterialInstance` _sm_watersurface 0 (`self.Ocean Material`) "None"))
  (set `self.Water Material` _returnvalue)
  (`SceneComponent.SetRelativeScale3D` _sm_watersurface (`KismetMathLibrary.MakeVector` (`self.Water Scale X`) (`self.Water Scale Y`) 1.0))
  (`MaterialInstanceDynamic.SetScalarParameterValue` _water_material "Shore Depth" (`self.Shore Depth`))
  (`MaterialInstanceDynamic.SetScalarParameterValue` _water_material "Wave Speed" (`self.Wave Speed`))
  (`MaterialInstanceDynamic.SetScalarParameterValue` _water_material "BaseOpacity" (`self.Base Opacity`))
  (`MaterialInstanceDynamic.SetScalarParameterValue` _water_material "Water Height" (.z (`SceneComponent.K2_GetComponentLocation` (`self.SM_WaterSurface`))))
  (`MaterialInstanceDynamic.SetScalarParameterValue` _water_material "Water Scale" (`self.Overall Water Scale`))
  (`MaterialInstanceDynamic.SetScalarParameterValue` _water_material "Variation Amount" (`self.Variation Amount`))
  (`MaterialInstanceDynamic.SetVectorParameterValue` _water_material "WaterColor A" (`self.Primary Water Color`))
  (`MaterialInstanceDynamic.SetVectorParameterValue` _water_material "WaterColor B" (`self.Secondary Water Color`))
  (`MaterialInstanceDynamic.SetScalarParameterValue` _water_material_2 "Water Depth" (`self.Depth Scale`))
  (`MaterialInstanceDynamic.SetVectorParameterValue` _water_material_2 "DeepWater" (`self.Deep Water Color`))
  (`MaterialInstanceDynamic.SetVectorParameterValue` _water_material_2 "ShallowWater" (`self.Shallow Water Color`)))
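; BP_Lamp_Medium is a cosmetic lamp prop for the AsianTemple environment, pairing a lamp mesh with a point light.
; It registers the mesh with its parent's material customization system, exposing named lamp tint and emissive colors.
; After the parent construction script runs, it optionally copies the tint color, not the emissive, to the point light.
; It has no active runtime event logic.
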(fn `ChildMaterialVariablesSetup`
  (set `self.MaterialCustomizations` (`|MakeArray` (make `/Game/changjing/AsianTemple/Blueprint/Structures/CustomizableParent/S_MaterialCustomization` (`|MakeArray` (`self.BP_Lamp_01a`)) (`|MakeArray` (make `/Game/changjing/AsianTemple/Blueprint/Structures/CustomizableParent/S_MaterialIdentity` "NewEnumerator0" 0 "None" (make `/Game/changjing/AsianTemple/Blueprint/Structures/CustomizableParent/S_MaterialParameterOptions` true "Lamp Tint Color" "Main_AlbedoTint" false "" "Main_TintColor_1" false "" "Main_TintColor_2" true "Lamp Emissive Color"))))))
  (`parent.ChildMaterialVariablesSetup`))

(fn `UserConstructionScript`
  (`parent.UserConstructionScript`)
  (if (`self.bSetPointLightColorToLampTintColor`)
    (`LightComponent.SetLightColor` (`self.PointLight`) (`BlueprintMapLibrary.Map_Find` (`self.ColorCustomizations`) (`.Main_AlbedoTint_CustomName_24_C9AC18E6474429253DA6C98B978F3173` (break `/Game/changjing/AsianTemple/Blueprint/Structures/CustomizableParent/S_MaterialParameterOptions` (`.OptionParameters_15_0A1F251F43E5A752387BA2BAD20AD891` (break `/Game/changjing/AsianTemple/Blueprint/Structures/CustomizableParent/S_MaterialIdentity` (`|GetArrayItem` (`.IndexIdentities_12_014E9DE24E22BF69DF2320BC0201BA45` (break `/Game/changjing/AsianTemple/Blueprint/Structures/CustomizableParent/S_MaterialCustomization` (`|GetArrayItem` (`self.MaterialCustomizations`)))))))))) true)))
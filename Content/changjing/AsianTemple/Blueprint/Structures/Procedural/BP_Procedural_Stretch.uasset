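; Procedural structure Blueprint that stretches a selected static mesh along a spline, one spline mesh per segment.
; The construction script picks the mesh by clamped index and bends each segment between neighboring spline points on a chosen forward axis.
; Tangents can optionally be clamped to the length from GetCorrectSizeForSegment on that axis.
; Each segment receives configurable collision and dynamic material instances carrying an albedo tint.
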(fn `UserConstructionScript`
  (locals (Local_createdStaticMeshComponent :type "SplineMeshComponent Object Reference") (Local_segmentIndex :type Integer) (Local_selectedStaticMesh :type "StaticMesh Object Reference"))
  (bind _local_segmentindex (`local.Local_segmentIndex`))
  (bind _local_createdstaticmeshcomponent (`local.Local_createdStaticMeshComponent`))
  (bind _local_createdstaticmeshcomponent_2 (`local.Local_createdStaticMeshComponent`))
  (bind _local_createdstaticmeshcomponent_3 (`local.Local_createdStaticMeshComponent`))
  (bind _mainspline (`self.MainSpline`))
  (bind (_sizevector_x _sizevector_y _sizevector_z) (`KismetMathLibrary.BreakVector` (`self.GetCorrectSizeForSegment` (`local.Local_selectedStaticMesh`))))
  (bind (_location _tangent) (`SplineComponent.GetLocationAndTangentAtSplinePoint` _mainspline _local_segmentindex "Local"))
  (bind (_location_2 _tangent_2) (`SplineComponent.GetLocationAndTangentAtSplinePoint` _mainspline (+ _local_segmentindex 1) "Local"))
  (bind _returnvalue (select `ESplineMeshAxis` (`self.ForwardAxis`) :`X` _sizevector_x :`Y` _sizevector_y :`Z` _sizevector_z))
  (`parent.UserConstructionScript`)
  (bind _output_get (set `self.StaticMeshSelection` (`KismetMathLibrary.Clamp` (`self.StaticMeshSelection`) 0 (- (`KismetArrayLibrary.Array_Length` (`self.StaticMeshes`)) 1))))
  (bind _output_get_2 (set `local.Local_selectedStaticMesh` (`|GetArrayItem` (`self.StaticMeshes`) _output_get)))
  (`/Engine/EditorBlueprintResources/StandardMacros.IsValid` _output_get_2
    (:`Is Valid`
      (for _index (range (+ (- (`SplineComponent.GetNumberOfSplinePoints` (`self.MainSpline`)) 2) 1))
        (set `local.Local_segmentIndex` _index)
        (bind _returnvalue_2 (`AddComponent|NODE_AddSplineMeshComponent-0`))
        (set `local.Local_createdStaticMeshComponent` _returnvalue_2)
        (`StaticMeshComponent.SetStaticMesh` _local_createdstaticmeshcomponent (`local.Local_selectedStaticMesh`))
        (`SplineMeshComponent.SetForwardAxis` _local_createdstaticmeshcomponent (`self.ForwardAxis`) true)
        (`SceneComponent.K2_AttachToComponent` _local_createdstaticmeshcomponent (`self.MainSpline`) "None" "KeepRelative" "KeepRelative" "KeepRelative" true)
        (`SplineMeshComponent.SetStartAndEnd` (`local.Local_createdStaticMeshComponent`) _location (select `bool` (`self.ClampTangent?`) :`false` _tangent :`true` (`KismetMathLibrary.ClampVectorSize` _tangent _returnvalue _returnvalue)) _location_2 (select `bool` (`self.ClampTangent?`) :`false` _tangent_2 :`true` (`KismetMathLibrary.ClampVectorSize` _tangent_2 _returnvalue _returnvalue)) true)
        (`PrimitiveComponent.SetCollisionEnabled` _local_createdstaticmeshcomponent_2 (`self.CollisionEnable`))
        (`PrimitiveComponent.SetCollisionObjectType` _local_createdstaticmeshcomponent_2 (`self.CollisionType`))
        (`StaticMeshComponent.SetForcedLodModel` (`local.Local_createdStaticMeshComponent`) 0)
        (for _index_2 (range (`PrimitiveComponent.GetNumMaterials` (`local.Local_createdStaticMeshComponent`)))
          (bind _returnvalue_3 (`PrimitiveComponent.CreateDynamicMaterialInstance` _local_createdstaticmeshcomponent_3 _index_2 (`PrimitiveComponent.GetMaterial` _local_createdstaticmeshcomponent_3 _index_2) "None"))
          (`MaterialInstanceDynamic.SetVectorParameterValue` _returnvalue_3 "Main_AlbedoTint" (`self.AlbedoTint`)))))))
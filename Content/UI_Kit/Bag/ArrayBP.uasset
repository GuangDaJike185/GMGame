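; ArrayBP is a battle formation actor that spawns partners and enemies at nine slot components in front, middle and back rows.
; The slot index selects the spawn transform and row Position; spawned units get AI initialised and register in the Global game instance, with enemy passives initialised afterwards.
; FormationPartner remembers each partner class's slot, so Revive respawns RevivePartner there with skill-grade-scaled HP and removes it from DeadPartner.
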(fn `Revive`
  (params (Skilllevel :type "/Game/AI/Structure/Level Enum" :default "NewEnumerator5"))
  (bind _revivepartner (`self.RevivePartner`))
  (bind _value (`BlueprintMapLibrary.Map_Find` (`self.Formation_Partner`) _revivepartner))
  (bind _returnvalue (select `int` _value :`0` (`self.前卫1`) :`1` (`self.前卫2`) :`2` (`self.前卫3`) :`3` (`self.中卫1`) :`4` (`self.中卫2`) :`5` (`self.中卫3`) :`6` (`self.后卫1`) :`7` (`self.后卫2`) :`8` (`self.后卫3`)))
  (bind _returnvalue_2 (`|SpawnActorFromClass` _revivepartner (`KismetMathLibrary.MakeTransform` (`SceneComponent.K2_GetComponentLocation` _returnvalue) (`SceneComponent.K2_GetComponentRotation` _returnvalue)) "Undefined" "OverrideRootScale" null (struct) null))
  (`/Game/AI/PartnerAI/PartnerParent.InitPartnerAI` _returnvalue_2)
  (`/Game/AI/AI_Base.InitAIBase` _returnvalue_2 (`/Game/AI/AI_Base.AI_Base` _returnvalue_2) (`/Game/AI/AI_Base.Mask` _returnvalue_2))
  (`self.以百分比的血量复活` _returnvalue_2 Skilllevel)
  (bind _asglobal (cast `/Game/Global/Global` (`GameplayStatics.GetGameInstance`)))
  (`KismetArrayLibrary.Array_AddUnique` (`/Game/Global/Global.PartnerAI` _asglobal) _returnvalue_2)
  (if (< _value 3)
    (set `/Game/AI/AI_Base.Position` "NewEnumerator0" _returnvalue_2)
    (elif (< _value 6)
      (set `/Game/AI/AI_Base.Position` "NewEnumerator1" _returnvalue_2)
      (else
        (set `/Game/AI/AI_Base.Position` "NewEnumerator2" _returnvalue_2))))
  (`KismetArrayLibrary.Array_RemoveItem` (`/Game/Global/Global.DeadPartner` _asglobal) (`self.RevivePartner`)))

(fn `SpawnEnemy`
  (params (EnemyArray :type "Array of /Game/AI/Enemy/EnemyParent Class Reference"))
  (bind _asglobal (cast `/Game/Global/Global` (`GameplayStatics.GetGameInstance`)))
  (bind _enemycombat (`/Game/Global/Global.EnemyCombat` _asglobal))
  (`KismetArrayLibrary.Array_Clear` _enemycombat)
  (for (_array_element _array_index) EnemyArray
    (if (`KismetSystemLibrary.IsValidClass` _array_element)
      (bind _returnvalue (select `int` _array_index :`0` (`self.前卫1`) :`1` (`self.前卫2`) :`2` (`self.前卫3`) :`3` (`self.中卫1`) :`4` (`self.中卫2`) :`5` (`self.中卫3`) :`6` (`self.后卫1`) :`7` (`self.后卫2`) :`8` (`self.后卫3`)))
      (bind _returnvalue_2 (`|SpawnActorFromClass` _array_element (`KismetMathLibrary.MakeTransform` (`SceneComponent.K2_GetComponentLocation` _returnvalue) (`SceneComponent.K2_GetComponentRotation` _returnvalue)) "Undefined" "OverrideRootScale" null (struct) null))
      (`/Game/AI/AI_Base.InitAIBase` _returnvalue_2 (`/Game/AI/AI_Base.AI_Base` _returnvalue_2) (`/Game/AI/AI_Base.Mask` _returnvalue_2))
      (bind _asglobal_2 (cast `/Game/Global/Global` (`GameplayStatics.GetGameInstance`)))
      (`KismetArrayLibrary.Array_Add` (`/Game/Global/Global.EnemyCombat` _asglobal_2) _returnvalue_2)
      (if (< _array_index 3)
        (set `/Game/AI/AI_Base.Position` "NewEnumerator0" _returnvalue_2)
        (elif (< _array_index 6)
          (set `/Game/AI/AI_Base.Position` "NewEnumerator1" _returnvalue_2)
          (else
            (set `/Game/AI/AI_Base.Position` "NewEnumerator2" _returnvalue_2))))))
  (for _array_element_2 _enemycombat
    (`/Game/AI/AI_Base.InitPassive` _array_element_2 _enemycombat)))

(fn `SpawnPartner`
  (params (ArrayIndex :type Integer) (PartnerClass :type "Actor Class Reference"))
  (bind _returnvalue (select `int` ArrayIndex :`0` (`self.前卫1`) :`1` (`self.前卫2`) :`2` (`self.前卫3`) :`3` (`self.中卫1`) :`4` (`self.中卫2`) :`5` (`self.中卫3`) :`6` (`self.后卫1`) :`7` (`self.后卫2`) :`8` (`self.后卫3`)))
  (bind _returnvalue_2 (`|SpawnActorFromClass` PartnerClass (`KismetMathLibrary.MakeTransform` (`SceneComponent.K2_GetComponentLocation` _returnvalue) (`SceneComponent.K2_GetComponentRotation` _returnvalue)) "Undefined" "OverrideRootScale" null null))
  (bind _aspartner_parent (cast `/Game/AI/PartnerAI/PartnerParent` _returnvalue_2))
  (`BlueprintMapLibrary.Map_Add` (`self.Formation_Partner`) PartnerClass ArrayIndex)
  (`/Game/AI/PartnerAI/PartnerParent.InitPartnerAI` _aspartner_parent)
  (`/Game/AI/AI_Base.InitAIBase` _aspartner_parent (`/Game/AI/AI_Base.AI_Base` _aspartner_parent) (`/Game/AI/AI_Base.Mask` _aspartner_parent))
  (bind _asglobal (cast `/Game/Global/Global` (`GameplayStatics.GetGameInstance`)))
  (`KismetArrayLibrary.Array_AddUnique` (`/Game/Global/Global.PartnerAI` _asglobal) _aspartner_parent)
  (if (< ArrayIndex 3)
    (set `/Game/AI/AI_Base.Position` "NewEnumerator0" _aspartner_parent)
    (elif (< ArrayIndex 6)
      (set `/Game/AI/AI_Base.Position` "NewEnumerator1" _aspartner_parent)
      (else
        (set `/Game/AI/AI_Base.Position` "NewEnumerator2" _aspartner_parent)))))

(fn `UserConstructionScript`)